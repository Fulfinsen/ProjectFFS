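; BP_TestItem is a test pickup item that implements an interaction interface.
; LookAt uses the item data component's row handle to fetch the item's data table row and returns a "Pick up" prompt with its name.
; Interact only prints "Added to inventory", and the other interaction getters return default or empty values.
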(event `/Game/Blueprints/Interfaces/BPI_Interact.Interact`
  (params (Caller :type "Actor Object Reference"))
  (`KismetSystemLibrary.PrintString` "Added to inventory"))

(fn `GetHoldDuration`
  (returns (Duration :type "Float (double-precision)"))
  (return 0.0))

(fn `GetInteractionLocation`
  (returns (Location :type "Vector Structure"))
  (return (0.0 0.0 0.0)))

(fn `GetInteractionPrompt`
  (returns (Value :type Text))
  (return ""))

(fn `GetInteractionType`
  (returns (Type :type "/Game/Blueprints/Interfaces/E_InteractionType Enum"))
  (return "NewEnumerator0"))

(fn `GetTaps`
  (returns (Taps :type Integer))
  (return 0))

(fn `LookAt`
  (returns (Message :type Text))
  (bind (_itemid_datatable _itemid_rowname) (break `DataTableRowHandle` (`/Game/Inventory/BP_ItemDataComponent.ItemID` (`self.BP_ItemDataComponent`))))
  (bind _returnvalue (`|GetDataTableRow` _itemid_datatable _itemid_rowname)
    (:`then`
      (return (`|FormatText` "Pick up {item}" (`.Name_2_B6F0023D4D83E0892D4F159CDAF29DAC` (break `/Game/Inventory/FItemStruct` _returnvalue)))))))

(fn `UserConstructionScript`)