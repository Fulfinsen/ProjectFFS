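; BP_ItemDataComponent is an actor component that makes its owning actor a pickup for the player's inventory.
; On Interact, it casts the caller to BP_FirstPersonCharacter and passes its data table row name and Quantity to BP_InventorySystem's AddToInventory, destroying the owner on success.
; The other interaction functions return empty, zero or first-enum values, and a disconnected weapon-equip path is parked for possible later use.
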(event `/Game/Blueprints/Interfaces/BPI_Interact.Interact`
  (params (Caller :type "Actor Object Reference"))
  (bind (_itemid_datatable _itemid_rowname) (break `DataTableRowHandle` (`self.ItemID`)))
  (bind _asbp_first_person_character (cast `/Game/FirstPerson/Blueprints/BP_FirstPersonCharacter` Caller))
  (bind _returnvalue (`Actor.GetComponentByClass` _asbp_first_person_character "/Game/Inventory/BP_InventorySystem.BP_InventorySystem_C"))
  (`/Engine/EditorBlueprintResources/StandardMacros.IsValid` _returnvalue
    (:`Is Valid`
      (bind _success (`/Game/Inventory/BP_InventorySystem.AddToInventory` _returnvalue _itemid_rowname (`self.Quantity`)))
      (if _success
        (`Actor.K2_DestroyActor` (`self.GetOwner`))))))

(fn `GetHoldDuration`
  (returns (Duration :type "Float (double-precision)"))
  (return 0.0))

(fn `GetInteractionLocation`
  (returns (Location :type "Vector Structure"))
  (return (0.0 0.0 0.0)))

(fn `GetInteractionPrompt`
  (returns (Value :type Text))
  (return ""))

(fn `GetInteractionType`
  (returns (Type :type "/Game/Blueprints/Interfaces/E_InteractionType Enum"))
  (return "NewEnumerator0"))

(fn `GetTaps`
  (returns (Taps :type Integer))
  (return 0))

(fn `LookAt`
  (returns (Message :type Text))
  (return ""))