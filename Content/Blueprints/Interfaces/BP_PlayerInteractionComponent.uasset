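; Player interaction component that lets a Character use nearby actors implementing BPI_Interact through press, hold or tap input.
; Capsule overlaps maintain the in-range list, and its last entry is the active interactable.
; A screen-space widget component created at BeginPlay shows that target's prompt at its interaction location or actor location.
; IA_Interact drives the interaction, using event dispatchers for hold timing and a counter for taps, both feeding widget progress.
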(event `self.ReceiveBeginPlay`
  (bind _ascharacter (cast `Character` (`self.GetOwner`)))
  (bind _capsulecomponent (`Character.CapsuleComponent` _ascharacter))
  (add `PrimitiveComponent.OnComponentBeginOverlap` _capsulecomponent (`|CreateDelegate` :!event `HandleCapsuleOverlapBegin`))
  (add `PrimitiveComponent.OnComponentEndOverlap` _capsulecomponent (`|CreateDelegate` :!event `HandleCapsuleOverlapEnd`))
  (bind _returnvalue (`|AddComponentByClass` :`self` (`self.GetOwner`) :`Class` "/Script/UMG.WidgetComponent" :`bManualAttachment` true))
  (`WidgetComponent.SetWidgetSpace` _returnvalue "Screen")
  (`WidgetComponent.SetDrawSize` _returnvalue (250.0 30.0))
  (set `self.InteractionWidgetComponent` _returnvalue))

(event `HandleCapsuleOverlapBegin`
  (params (OverlappedComponent :type "PrimitiveComponent Object Reference") (OtherActor :type "Actor Object Reference") (OtherComp :type "PrimitiveComponent Object Reference") (OtherBodyIndex :type Integer) (bFromSweep :type Boolean) (SweepResult :type "HitResult Structure (by ref)"))
  (if (`KismetSystemLibrary.DoesImplementInterface` OtherActor "/Game/Blueprints/Interfaces/BPI_Interact.BPI_Interact_C")
    (`KismetArrayLibrary.Array_AddUnique` (`self.InteractablesInRange`) OtherActor)
    (`self.RenderInteractionWidget`)))

(event `HandleCapsuleOverlapEnd`
  (params (OverlappedComponent :type "PrimitiveComponent Object Reference") (OtherActor :type "Actor Object Reference") (OtherComp :type "PrimitiveComponent Object Reference") (OtherBodyIndex :type Integer))
  (if (`KismetSystemLibrary.DoesImplementInterface` OtherActor "/Game/Blueprints/Interfaces/BPI_Interact.BPI_Interact_C")
    (if (== OtherActor (`self.GetActiveInteractable`))
      (`self.ResetInteractionState`))
    (`KismetArrayLibrary.Array_RemoveItem` (`self.InteractablesInRange`) OtherActor)
    (`self.RenderInteractionWidget`)))

(event `EnhancedInput|/Game/Input/Actions/IA_Interact`
  (params (ActionValue :type Boolean) (ElapsedSeconds :type "Float (double-precision)") (TriggeredSeconds :type "Float (double-precision)") (InputAction :type "InputAction Object Reference" :default "/Game/Input/Actions/IA_Interact.IA_Interact"))
  (:`Started`
    (`self.InteractBegin`))
  (:`Ongoing`
    (`self.OnInteractionPressOnGoing` ElapsedSeconds))
  (:`Canceled`
    (clear `self.OnInteractionPressOnGoing` :!label _label)
    (`self.OnInteractionEnded`))
  (:`Completed`
    (goto _label)))

(event `InteractWithActiveInteractable`
  (message `/Game/Blueprints/Interfaces/BPI_Interact.Interact` (`self.GetActiveInteractable`) (`self.GetOwner`))
  (`self.RenderInteractionWidget`)
  (`self.ResetInteractionState`))

(event `InteractBegin`
  (bind _activeinteractable (`self.GetActiveInteractable`))
  (`/Engine/EditorBlueprintResources/StandardMacros.IsValid` _activeinteractable
    (:`Is Valid`
      (bind _type (message `/Game/Blueprints/Interfaces/BPI_Interact.GetInteractionType` _activeinteractable))
      (switch `/Game/Blueprints/Interfaces/E_InteractionType` _type
        (:`NewEnumerator0`
          (`self.InteractWithActiveInteractable`))
        (:`NewEnumerator1`
          (add `self.OnInteractionPressOnGoing` (`|CreateDelegate` :!event `InteractionHoldOngoing`))
          (add `self.OnInteractionEnded` (delegate `ResetWidgetProgress`)))
        (:`NewEnumerator2`
          (`self.InteractionTap`))))))

(event `ResetWidgetProgress`
  (bind _interactionwidgetref (`self.InteractionWidgetRef`)
    (:`then`
      (`/Game/Blueprints/Interfaces/WBP_InteractionWiedget.SetProgressPercent` _interactionwidgetref 0.0)
      (remove `self.OnInteractionEnded` (delegate `ResetWidgetProgress`)))
    (:`else`)))

(event `InteractionHoldOngoing` :!signature `self.OnInteractionPressOnGoing`
  (params (ElapsedSeconds :type "Float (double-precision)"))
  (bind _activeinteractable (`self.GetActiveInteractable`))
  (`/Engine/EditorBlueprintResources/StandardMacros.IsValid` _activeinteractable
    (:`Is Valid`
      (bind _duration (message `/Game/Blueprints/Interfaces/BPI_Interact.GetHoldDuration` _activeinteractable))
      (bind _interactionwidgetref (`self.InteractionWidgetRef`)
        (:`then`
          (`/Game/Blueprints/Interfaces/WBP_InteractionWiedget.SetProgressPercent` _interactionwidgetref (mod ElapsedSeconds _duration)))
        (:`else`
          _))
      (if (> ElapsedSeconds _duration)
        (`self.InteractWithActiveInteractable`)
        (remove `self.OnInteractionPressOnGoing` (delegate `InteractionHoldOngoing`))
        (`KismetSystemLibrary.PrintString` "Unbinded")))))

(event `InteractionTap`
  (`/Engine/EditorBlueprintResources/StandardMacros.IncrementInt` (`self.CurrentTapCount`)
    (:`  `
      (bind _taps (message `/Game/Blueprints/Interfaces/BPI_Interact.GetTaps` (`self.GetActiveInteractable`)))
      (if (<= _taps 0)
        (`self.InteractWithActiveInteractable`)
        (else
          (bind _interactionwidgetref (`self.InteractionWidgetRef`)
            (:`then`
              (`/Game/Blueprints/Interfaces/WBP_InteractionWiedget.SetProgressPercent` _interactionwidgetref (/ (`self.CurrentTapCount`) _taps))
              (if (>= (`self.CurrentTapCount`) _taps)
                (`self.InteractWithActiveInteractable`)))
            (:`else`)))))))

(fn `GetActiveInteractable`
  (returns (ActiveInteractable :type "Actor Object Reference"))
  (bind _interactablesinrange (`self.InteractablesInRange`))
  (return (`|GetArrayItem` _interactablesinrange (`KismetArrayLibrary.Array_LastIndex` _interactablesinrange))))

(fn `RenderInteractionWidget`
  (bind _activeinteractable (`self.GetActiveInteractable`))
  (bind _activeinteractable_2 (`self.GetActiveInteractable`))
  (bind _interactionwidgetcomponent (`self.InteractionWidgetComponent`))
  (`/Engine/EditorBlueprintResources/StandardMacros.IsValid` _activeinteractable
    (:`Is Valid`
      (bind _type (message `/Game/Blueprints/Interfaces/BPI_Interact.GetInteractionType` _activeinteractable))
      (bind _value (message `/Game/Blueprints/Interfaces/BPI_Interact.GetInteractionPrompt` _activeinteractable))
      (bind _returnvalue (`|CreateWidget` "/Game/Blueprints/Interfaces/WBP_InteractionWiedget.WBP_InteractionWiedget_C" null _type _value))
      (set `self.InteractionWidgetRef` _returnvalue)
      (`WidgetComponent.SetWidget` _interactionwidgetcomponent _returnvalue)
      (bind _location (message `/Game/Blueprints/Interfaces/BPI_Interact.GetInteractionLocation` _activeinteractable_2))
      (`SceneComponent.K2_SetWorldLocation` _interactionwidgetcomponent (`KismetMathLibrary.SelectVector` (`Actor.K2_GetActorLocation` _activeinteractable_2) _location (`KismetMathLibrary.Vector_IsZero` _location)) false false))
    (:`Is Not Valid`
      (`WidgetComponent.SetWidget` (`self.InteractionWidgetComponent`) null))))

(fn `ResetInteractionState`
  (remove `self.OnInteractionPressOnGoing` (`|CreateDelegate` :!event `InteractionHoldOngoing`))
  (set `self.CurrentTapCount` 0))