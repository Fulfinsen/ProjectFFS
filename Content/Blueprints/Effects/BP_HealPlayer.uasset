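; BP_HealPlayer is a one-shot effect actor that heals the player as soon as it spawns.
; On BeginPlay it casts player 0's character to BP_FirstPersonCharacter and adds its heal amount to current health, clamped between zero and max health.
; It then calls the character's health update event, destroys itself and prints a debug message; a failed cast leaves the actor in place.
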(event `self.ReceiveBeginPlay`
  (bind _asbp_first_person_character (cast `/Game/FirstPerson/Blueprints/BP_FirstPersonCharacter` (`GameplayStatics.GetPlayerCharacter` 0)))
  (set `/Game/FirstPerson/Blueprints/BP_FirstPersonCharacter.CurrentHealth` (`KismetMathLibrary.FClamp` (+ (`/Game/FirstPerson/Blueprints/BP_FirstPersonCharacter.CurrentHealth` _asbp_first_person_character) (`self.HealAmmount`)) 0.0 (`/Game/FirstPerson/Blueprints/BP_FirstPersonCharacter.MaxHealth` _asbp_first_person_character)) _asbp_first_person_character)
  (`/Game/FirstPerson/Blueprints/BP_FirstPersonCharacter.E_UpdateHealth` _asbp_first_person_character (`/Game/FirstPerson/Blueprints/BP_FirstPersonCharacter.CurrentHealth` _asbp_first_person_character) (`/Game/FirstPerson/Blueprints/BP_FirstPersonCharacter.MaxHealth` _asbp_first_person_character))
  (`self.K2_DestroyActor`)
  (`KismetSystemLibrary.PrintString` "PlayerHealed"))

(fn `UserConstructionScript`
  (`parent.UserConstructionScript`))