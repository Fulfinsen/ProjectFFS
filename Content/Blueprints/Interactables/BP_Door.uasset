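; BP_Door is an interactable hinged door that toggles open and closed when interacted with.
; Interact checks IsOpen and calls OpenDoor or CloseDoor, which play or reverse a timeline that drives the Door component's yaw.
; Interaction getter functions supply the world location, a state-dependent prompt, the interaction type, and zero hold duration and taps.
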(event `OpenDoor`
  (set `self.isOpen` true)
  (bind (_direction _zrotation) (`Timeline|OpenDoorTimeline` :!label _label)
    (:`Update`
      (`SceneComponent.K2_SetRelativeRotation` (`self.Door`) (`KismetMathLibrary.MakeRotator` 0.0 0.0 _zrotation) false false))))

(event `CloseDoor`
  (set `self.isOpen` false)
  (goto _label :!via `Reverse`))

(event `/Game/Blueprints/Interfaces/BPI_Interact.Interact`
  (params (Caller :type "Actor Object Reference"))
  (if (`self.isOpen`)
    (`self.CloseDoor`)
    (else
      (`self.OpenDoor`))))

(fn `GetHoldDuration`
  (returns (Duration :type "Float (double-precision)"))
  (return 0.0))

(fn `GetInteractionLocation`
  (returns (Location :type "Vector Structure"))
  (return (`SceneComponent.K2_GetComponentLocation` (`self.InteractionLocation`))))

(fn `GetInteractionPrompt`
  (returns (Value :type Text))
  (return (select `bool` (`self.isOpen`) :`false` "to open the door" :`true` "to close the door" :!type "Text")))

(fn `GetInteractionType`
  (returns (Type :type "/Game/Blueprints/Interfaces/E_InteractionType Enum"))
  (return "NewEnumerator0"))

(fn `GetTaps`
  (returns (Taps :type Integer))
  (return 0))

(fn `LookAt`
  (returns (Message :type Name))
  (return "None"))

(fn `UserConstructionScript`)