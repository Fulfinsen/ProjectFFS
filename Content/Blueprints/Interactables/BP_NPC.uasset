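; Interactable NPC that shows a "to talk" prompt and turns to face whoever interacts with it.
; The Interact event sets the actor's rotation instantly to the look-at yaw toward the caller; no dialogue logic is present here.
; Getter functions supply the interaction type, prompt, zero hold duration and taps, and a world location taken from InteractionLocation.
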(event `/Game/Blueprints/Interfaces/BPI_Interact.Interact`
  (params (Caller :type "Actor Object Reference"))
  (bind (_returnvalue_roll _returnvalue_pitch _returnvalue_yaw) (`KismetMathLibrary.BreakRotator` (`KismetMathLibrary.FindLookAtRotation` (`self.K2_GetActorLocation`) (`self.K2_GetActorLocation` Caller))))
  (`self.K2_SetActorRotation` (`KismetMathLibrary.MakeRotator` 0.0 0.0 _returnvalue_yaw)))

(fn `GetHoldDuration`
  (returns (Duration :type "Float (double-precision)"))
  (return 0.0))

(fn `GetInteractionLocation`
  (returns (Location :type "Vector Structure"))
  (return (`SceneComponent.K2_GetComponentLocation` (`self.InteractionLocation`))))

(fn `GetInteractionPrompt`
  (returns (Value :type Text))
  (return "to talk"))

(fn `GetInteractionType`
  (returns (Type :type "/Game/Blueprints/Interfaces/E_InteractionType Enum"))
  (return "NewEnumerator0"))

(fn `GetTaps`
  (returns (Taps :type Integer))
  (return 0))

(fn `UserConstructionScript`)