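; BP_Chest is an interactable container the player can open, offering the prompt "to open the chest".
; On Interact, it casts player controller 0 to BP_FirstPersonPlayerController and has its HUD show the container using the chest's BPInventorySystem.
; Its interaction functions return fixed values: the first interaction type, zero hold duration and taps, a zero location and empty look-at text.
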(event `/Game/Blueprints/Interfaces/BPI_Interact.Interact`
  (params (Caller :type "Actor Object Reference"))
  (bind _asbp_first_person_player_controller (cast `/Game/FirstPerson/Blueprints/BP_FirstPersonPlayerController` (`GameplayStatics.GetPlayerController` 0)))
  (`/Game/UserInterfaces/WBP_PlayerHUD.ShowContainer` (`/Game/FirstPerson/Blueprints/BP_FirstPersonPlayerController.HUD` _asbp_first_person_player_controller) (`self.BP_InventorySystem`)))

(fn `GetHoldDuration`
  (returns (Duration :type "Float (double-precision)"))
  (return 0.0))

(fn `GetInteractionLocation`
  (returns (Location :type "Vector Structure"))
  (return (0.0 0.0 0.0)))

(fn `GetInteractionPrompt`
  (returns (Value :type Text))
  (return "to open the chest"))

(fn `GetInteractionType`
  (returns (Type :type "/Game/Blueprints/Interfaces/E_InteractionType Enum"))
  (return "NewEnumerator0"))

(fn `GetTaps`
  (returns (Taps :type Integer))
  (return 0))

(fn `LookAt`
  (returns (Message :type Text))
  (return ""))

(fn `UserConstructionScript`)