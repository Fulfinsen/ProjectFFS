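; BP_PickUp is an interactable pickup that destroys itself when interacted with.
; Interact prints an inventory message, plays a crowbar sound at its location and destroys the actor, without storing any item.
; The message's names are swapped, with the caller as the item and the pickup as the owner.
; Getters expose hold duration and interaction type, while prompt, look-at, tap count and location return empty or zero values.
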(event `/Game/Blueprints/Interfaces/BPI_Interact.Interact`
  (params (Caller :type "Actor Object Reference"))
  (`KismetSystemLibrary.PrintString` (`KismetTextLibrary.Conv_TextToString` (`|FormatText` "Added {ItemName} to the invetory of {ActorName}" (`KismetSystemLibrary.GetDisplayName` Caller) (`KismetSystemLibrary.GetDisplayName` self))))
  (`GameplayStatics.PlaySoundAtLocation` "/Game/Interaction/Sounds/Cue/Attack/Cue_Crowbar_Attack.Cue_Crowbar_Attack" (`self.K2_GetActorLocation`) (struct) 1.0 1.0 0.0 null null null null)
  (`self.K2_DestroyActor`))

(fn `GetHoldDuration`
  (returns (Duration :type "Float (double-precision)"))
  (return (`self.HoldDuration`)))

(fn `GetInteractionLocation`
  (returns (Location :type "Vector Structure"))
  (return (0.0 0.0 0.0)))

(fn `GetInteractionPrompt`
  (returns (Value :type Text))
  (return ""))

(fn `GetInteractionType`
  (returns (Type :type "/Game/Blueprints/Interfaces/E_InteractionType Enum"))
  (return (`self.InteractionType`)))

(fn `GetTaps`
  (returns (Taps :type Integer))
  (return 0))

(fn `LookAt`
  (returns (Message :type Text))
  (return ""))

(fn `UserConstructionScript`)