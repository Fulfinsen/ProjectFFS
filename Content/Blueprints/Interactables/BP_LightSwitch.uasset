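; BP_LightSwitch is an interactable light switch that toggles its PointLight's visibility on each Interact event.
; It answers interaction queries with a fixed type and tap count, leaving prompt, look-at text, location and hold duration empty or zero.
; Interact branches on IsOn to LightOn or LightOff, but each rewrites the same value, so IsOn never flips and only ToggleVisibility changes the light.
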(event `/Game/Blueprints/Interfaces/BPI_Interact.Interact`
  (params (Caller :type "Actor Object Reference"))
  (if (`self.isOn`)
    (`self.LightOn`)
    (else
      (`self.LightOff`))))

(event `LightOn`
  (set `self.isOn` true)
  (`SceneComponent.ToggleVisibility` (`self.PointLight`) false))

(event `LightOff`
  (set `self.isOn` false)
  (`SceneComponent.ToggleVisibility` (`self.PointLight`) false))

(fn `GetHoldDuration`
  (returns (Duration :type "Float (double-precision)"))
  (return 0.0))

(fn `GetInteractionLocation`
  (returns (Location :type "Vector Structure"))
  (return (0.0 0.0 0.0)))

(fn `GetInteractionPrompt`
  (returns (Value :type Text))
  (return ""))

(fn `GetInteractionType`
  (returns (Type :type "/Game/Blueprints/Interfaces/E_InteractionType Enum"))
  (return "NewEnumerator2"))

(fn `GetTaps`
  (returns (Taps :type Integer))
  (return 4))

(fn `LookAt`
  (returns (Message :type Text))
  (return ""))

(fn `UserConstructionScript`)