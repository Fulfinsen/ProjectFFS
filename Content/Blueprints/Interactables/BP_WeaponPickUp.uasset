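; BP_WeaponPickUp is an interactable world pickup that gives the player a melee weapon.
; On BeginPlay it destroys itself if its PickupID is in the game instance's saved collected pickups, otherwise it sets its display mesh from its DT_MeleeWeapons row.
; On interact it records the PickupID in that save data, adds the weapon row name to the first-person character's inventory component and destroys itself.
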(event `self.ReceiveBeginPlay`
  (bind _asbp_fulfinsen_game_instance (cast `/Game/Blueprints/BP_FulfinsenGameInstance` (`GameplayStatics.GetGameInstance`)))
  (if (`BlueprintSetLibrary.Set_Contains` (`/Game/Blueprints/SaveSystem/BP_SaveData_PlayerData.CollectedPickUps` (`/Game/Blueprints/BP_FulfinsenGameInstance.As BP Save Data Player Data` _asbp_fulfinsen_game_instance)) (`self.PickupID`))
    (`self.K2_DestroyActor`)
    (else
      (bind _returnvalue (`|GetDataTableRow` "/Game/Blueprints/Structures/DT_MeleeWeapons.DT_MeleeWeapons" (`self.WeaponRowName`))
        (:`then`
          (`StaticMeshComponent.SetStaticMesh` (`self.WeaponDisplayMesh`) (`.WeaponMesh_14_59134104402D201C4BD8D3A0839A654F` (break `/Game/Blueprints/Structures/S_MeleeWeaponsStats` _returnvalue))))))))

(event `/Game/Blueprints/Interfaces/BPI_Interact.Interact`
  (params (Caller :type "Actor Object Reference"))
  (bind _asbp_first_person_character (cast `/Game/FirstPerson/Blueprints/BP_FirstPersonCharacter` Caller))
  (bind _asbp_fulfinsen_game_instance (cast `/Game/Blueprints/BP_FulfinsenGameInstance` (`GameplayStatics.GetGameInstance`)))
  (`BlueprintSetLibrary.Set_Add` (`/Game/Blueprints/SaveSystem/BP_SaveData_PlayerData.CollectedPickUps` (`/Game/Blueprints/BP_FulfinsenGameInstance.As BP Save Data Player Data` _asbp_fulfinsen_game_instance)) (`self.PickupID`))
  (`/Game/Inventory/BP_InventorySystem.AddToInventory` (`self.GetComponentByClass` _asbp_first_person_character "/Game/Inventory/BP_InventorySystem.BP_InventorySystem_C") (`self.WeaponRowName`) 1)
  (`KismetSystemLibrary.PrintString` "Weapon picked")
  (`self.K2_DestroyActor`))

(fn `GetHoldDuration`
  (returns (Duration :type "Float (double-precision)"))
  (return 0.0))

(fn `GetInteractionLocation`
  (returns (Location :type "Vector Structure"))
  (return (0.0 0.0 0.0)))

(fn `GetInteractionPrompt`
  (returns (Value :type Text))
  (return "to pick up"))

(fn `GetInteractionType`
  (returns (Type :type "/Game/Blueprints/Interfaces/E_InteractionType Enum"))
  (return "NewEnumerator0"))

(fn `GetTaps`
  (returns (Taps :type Integer))
  (return 0))

(fn `LookAt`
  (returns (Message :type Text))
  (return "Weapon Picked up"))

(fn `UserConstructionScript`)