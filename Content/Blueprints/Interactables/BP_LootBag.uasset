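; BP_LootBag is an interactable loot container with an inventory component that records itself in level save data.
; On BeginPlay it adds its class and transform to the game mode's ActorsAdded and saves the level slot.
; When an inventory update leaves it empty, it closes the player's HUD menu, registers itself in ActorsRemoved without saving the slot, and destroys itself.
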(event `self.ReceiveBeginPlay`
  (`parent.ReceiveBeginPlay`)
  (bind _asbp_first_person_game_mode (cast `/Game/FirstPerson/Blueprints/BP_FirstPersonGameMode` (`GameplayStatics.GetGameMode`)))
  (bind _as_bp_save_data_level_data (`/Game/FirstPerson/Blueprints/BP_FirstPersonGameMode.As BP Save Data Level Data` _asbp_first_person_game_mode))
  (`BlueprintMapLibrary.Map_Add` (`/Game/Blueprints/SaveSystem/BP_SaveData_LevelData.ActorsAdded` _as_bp_save_data_level_data) (`|ConvertAsset` (`GameplayStatics.GetObjectClass` self)) (`self.GetTransform`))
  (`GameplayStatics.SaveGameToSlot` _as_bp_save_data_level_data (`/Game/FirstPerson/Blueprints/BP_FirstPersonGameMode.LevelDataSlot` _asbp_first_person_game_mode)))

(event `self.ReceiveDestroyed`)

(event `self.BP_InventorySystem.OnInventoryUpdated`
  (if (<= (`/Game/Inventory/BP_InventorySystem.GetQuantity` (`self.BP_InventorySystem`)) 0)
    (bind _asbp_first_person_player_controller (cast `/Game/FirstPerson/Blueprints/BP_FirstPersonPlayerController` (`GameplayStatics.GetPlayerController` 0)))
    (`Widget.RemoveFromParent` (`/Game/UserInterfaces/WBP_PlayerHUD.Menu` (`/Game/FirstPerson/Blueprints/BP_FirstPersonPlayerController.HUD` _asbp_first_person_player_controller)))
    (bind _asbp_first_person_game_mode (cast `/Game/FirstPerson/Blueprints/BP_FirstPersonGameMode` (`GameplayStatics.GetGameMode`)))
    (`KismetArrayLibrary.Array_AddUnique` (`/Game/Blueprints/SaveSystem/BP_SaveData_LevelData.ActorsRemoved` (`/Game/FirstPerson/Blueprints/BP_FirstPersonGameMode.As BP Save Data Level Data` _asbp_first_person_game_mode)) (`|ConvertAsset` self))
    (`self.K2_DestroyActor`)))

(fn `UserConstructionScript`
  (`parent.UserConstructionScript`))